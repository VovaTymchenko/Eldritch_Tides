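; Shooting-target dummy that slides back and forth and awards points to the player when hit by first-person projectiles.
; On BeginPlay it caches the player character and records its start location, then two chained timelines lerp it endlessly between that point and a hardcoded Y position.
; Head, Body, RightArm and LeftArm overlaps with a projectile each add a different score to the character's Points.
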(event `self.ReceiveBeginPlay`
  (bind (_returnvalue_x _returnvalue_y _returnvalue_z) (`KismetMathLibrary.BreakVector` (`self.K2_GetActorLocation`)))
  ;[1 1 1] Target movement back and forth
  (set `self.Start` (`KismetMathLibrary.MakeVector` _returnvalue_x _returnvalue_y _returnvalue_z))
  (set `self.End` (`KismetMathLibrary.MakeVector` _returnvalue_x 2758.431124 _returnvalue_z))
  (bind _asbp_first_person_character (cast `/Game/FirstPerson/Blueprints/BP_FirstPersonCharacter` (`GameplayStatics.GetPlayerCharacter` 0)))
  (set `self.Char Ref` _asbp_first_person_character)
  (bind (_direction _move) (`Timeline|Move` :!via `PlayFromStart` :!label _label)
    (:`Update`
      (`self.K2_SetActorRelativeLocation` (`KismetMathLibrary.VLerp` (`self.Start`) (`self.End`) _move)))
    (:`Finished`
      (bind (_direction_2 _move_2) (`Timeline|Move Back` :!via `ReverseFromEnd`)
        (:`Update`
          (`self.K2_SetActorRelativeLocation` (`KismetMathLibrary.VLerp` (`self.Start`) (`self.End`) _move_2)))
        (:`Finished`
          (goto _label :!via `PlayFromStart`))))))

(event `self.Head.OnComponentBeginOverlap`
  (params (OverlappedComponent :type "PrimitiveComponent Object Reference") (OtherActor :type "Actor Object Reference") (OtherComp :type "PrimitiveComponent Object Reference") (OtherBodyIndex :type Integer) (bFromSweep :type Boolean) (SweepResult :type "HitResult Structure (by ref)"))
  (bind _char_ref (`self.Char Ref`))
  ;[1 1 1] Points system for different hit points
  (cast `/Game/FirstPerson/Blueprints/BP_FirstPersonProjectile` OtherActor)
  (set `/Game/FirstPerson/Blueprints/BP_FirstPersonCharacter.Points` (+ (`/Game/FirstPerson/Blueprints/BP_FirstPersonCharacter.Points` _char_ref) 5) _char_ref))

(event `self.Body.OnComponentBeginOverlap`
  (params (OverlappedComponent :type "PrimitiveComponent Object Reference") (OtherActor :type "Actor Object Reference") (OtherComp :type "PrimitiveComponent Object Reference") (OtherBodyIndex :type Integer) (bFromSweep :type Boolean) (SweepResult :type "HitResult Structure (by ref)"))
  (bind _char_ref (`self.Char Ref`))
  ;[1 1 1] Points system for different hit points
  (cast `/Game/FirstPerson/Blueprints/BP_FirstPersonProjectile` OtherActor)
  (set `/Game/FirstPerson/Blueprints/BP_FirstPersonCharacter.Points` (+ (`/Game/FirstPerson/Blueprints/BP_FirstPersonCharacter.Points` _char_ref) 10) _char_ref))

(event `self.RightArm.OnComponentBeginOverlap`
  (params (OverlappedComponent :type "PrimitiveComponent Object Reference") (OtherActor :type "Actor Object Reference") (OtherComp :type "PrimitiveComponent Object Reference") (OtherBodyIndex :type Integer) (bFromSweep :type Boolean) (SweepResult :type "HitResult Structure (by ref)"))
  (bind _char_ref (`self.Char Ref`))
  ;[1 1 1] Points system for different hit points
  (cast `/Game/FirstPerson/Blueprints/BP_FirstPersonProjectile` OtherActor)
  (set `/Game/FirstPerson/Blueprints/BP_FirstPersonCharacter.Points` (+ (`/Game/FirstPerson/Blueprints/BP_FirstPersonCharacter.Points` _char_ref) 7) _char_ref))

(event `self.LeftArm.OnComponentBeginOverlap`
  (params (OverlappedComponent :type "PrimitiveComponent Object Reference") (OtherActor :type "Actor Object Reference") (OtherComp :type "PrimitiveComponent Object Reference") (OtherBodyIndex :type Integer) (bFromSweep :type Boolean) (SweepResult :type "HitResult Structure (by ref)"))
  (bind _char_ref (`self.Char Ref`))
  ;[1 1 1] Points system for different hit points
  (cast `/Game/FirstPerson/Blueprints/BP_FirstPersonProjectile` OtherActor)
  (set `/Game/FirstPerson/Blueprints/BP_FirstPersonCharacter.Points` (+ (`/Game/FirstPerson/Blueprints/BP_FirstPersonCharacter.Points` _char_ref) 6) _char_ref))

(fn `UserConstructionScript`)