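; Ooze bomb projectile for the ooze spell, launched along the player's view and leaving an ooze decal.
; On BeginPlay it casts the player pawn to BP_FirstPersonCharacter and applies a velocity-change impulse to OozeBomb along the first-person camera's forward vector.
; After a short fixed delay, rather than on impact, it spawns OozeDecal_BP at the bomb's location with a fixed rotation and destroys itself.
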(event `self.ReceiveBeginPlay`
  (bind _ooze_bomb (`self.Ooze_Bomb`))
  (bind _asbp_first_person_character (cast `/Game/FirstPerson/Blueprints/BP_FirstPersonCharacter` (`GameplayStatics.GetPlayerPawn` 0)))
  (`PrimitiveComponent.AddImpulse` _ooze_bomb (* (`SceneComponent.GetForwardVector` (`/Game/FirstPerson/Blueprints/BP_FirstPersonCharacter.FirstPersonCamera` _asbp_first_person_character)) 1500.0) "None" true)
  (`KismetSystemLibrary.Delay` 1.5)
  (`|SpawnActorFromClass` "/Game/OozeSpell/OozeDecal_BP.OozeDecal_BP_C" (`KismetMathLibrary.MakeTransform` (`SceneComponent.K2_GetComponentLocation` _ooze_bomb) (struct :`Pitch` 90.0)) "Undefined" "OverrideRootScale" null null)
  (`self.K2_DestroyActor`))

(fn `UserConstructionScript`)