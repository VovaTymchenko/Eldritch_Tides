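; Flashbang_BP is a thrown flashbang spell actor that goes off on the first-person player character after a short fuse.
; On BeginPlay it launches its Sphere along the player camera's forward vector and adds a random angular impulse for tumble.
; After a fixed delay it calls the character's Flashbang function with a distance and the sphere's world location, then destroys itself.
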(event `self.ReceiveBeginPlay`
  (bind _sphere (`self.Sphere`))
  (bind _asbp_first_person_character (cast `/Game/Blueprints/BP_FirstPersonCharacter` (`GameplayStatics.GetPlayerPawn` 0)))
  (`PrimitiveComponent.AddImpulse` _sphere (* (`SceneComponent.GetForwardVector` (`/Game/Blueprints/BP_FirstPersonCharacter.FirstPersonCamera` _asbp_first_person_character)) 700.0) "None" true)
  (`PrimitiveComponent.AddAngularImpulseInDegrees` _sphere (* (`KismetMathLibrary.RandomUnitVector`) 350.0) "None" false)
  (`KismetSystemLibrary.Delay` 3.0)
  (`/Game/Blueprints/BP_FirstPersonCharacter.Flashbang` _asbp_first_person_character (`self.GetDistanceTo` _asbp_first_person_character null) (`SceneComponent.K2_GetComponentLocation` _sphere))
  (`self.K2_DestroyActor`))

(fn `UserConstructionScript`)