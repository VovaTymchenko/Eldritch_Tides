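; BP_BULLET is a projectile actor that deals damage to training dummies on hit.
; Its Hit event subtracts Damage from the struck BP_Training_Dummy's Health and prints the result.
; The same branch then takes a fixed amount off the player character's Health as a health bar test.
; Disconnected nodes hold unused logic for halting the bullet, attaching it to what it hit and destroying it after a delay.
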(event `self.ReceiveHit`
  (params (MyComp :type "PrimitiveComponent Object Reference") (Other :type "Actor Object Reference") (OtherComp :type "PrimitiveComponent Object Reference") (bSelfMoved :type Boolean) (HitLocation :type "Vector Structure") (HitNormal :type "Vector Structure") (NormalImpulse :type "Vector Structure") (Hit :type "HitResult Structure (by ref)"))
  ;[1 1 1] Deal Damage
  (`|ExecutionSequence`
    (:`then_0`
      (bind _asbp_training_dummy (cast `/Game/Blueprints/BP_Training_Dummy` (`.HitActor` (`GameplayStatics.BreakHitResult` Hit))))
      (set `/Game/Blueprints/BP_Training_Dummy.Health` (- (`/Game/Blueprints/BP_Training_Dummy.Health` _asbp_training_dummy) (`self.Damage`)) _asbp_training_dummy)
      (`KismetSystemLibrary.PrintString` (`KismetStringLibrary.Conv_DoubleToString` (`/Game/Blueprints/BP_Training_Dummy.Health` _asbp_training_dummy)))
      ;[1 1 1] Character HealthBar test
      (bind _asbp_first_person_character (cast `/Game/Blueprints/BP_FirstPersonCharacter` (`GameplayStatics.GetPlayerCharacter` 0)))
      (set `/Game/Blueprints/BP_FirstPersonCharacter.Health` (- (`/Game/Blueprints/BP_FirstPersonCharacter.Health` _asbp_first_person_character) 10.0) _asbp_first_person_character))))

(fn `UserConstructionScript`)