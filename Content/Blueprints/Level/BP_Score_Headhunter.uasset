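; BP_Score_Headhunter is a level interactable that lets the player view a scoreboard.
; Player overlap sets an interaction-zone flag and highlights its Sphere through custom depth rendering.
; The ToggleScoreboard event, when called inside the zone, creates and shows a WB_Scoreboard widget or removes the one already on screen.
; Leaving the zone clears the highlight and closes any open scoreboard.
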(event `self.ReceiveActorBeginOverlap`
  (params (OtherActor :type "Actor Object Reference"))
  (if (== OtherActor (`GameplayStatics.GetPlayerCharacter` 0))
    (`PrimitiveComponent.SetRenderCustomDepth` (`self.Sphere`) true)
    (set `self.inInteractionZone` true)))

(event `self.ReceiveActorEndOverlap`
  (params (OtherActor :type "Actor Object Reference"))
  (if (== OtherActor (`GameplayStatics.GetPlayerCharacter` 0))
    (`PrimitiveComponent.SetRenderCustomDepth` (`self.Sphere`) false)
    (set `self.inInteractionZone` false)
    (if (`self.isWidgetOn`)
      (`Widget.RemoveFromParent` (`self.scoreboardRef`) :!label _label)
      (set `self.isWidgetOn` false))))

(event `Toggle Scoreboard`
  (if (`self.inInteractionZone`)
    (if (`self.isWidgetOn`)
      (goto _label)
      (else
        (bind _returnvalue (`|CreateWidget` "/Game/UI/WB_Scoreboard.WB_Scoreboard_C"))
        (bind _output_get (set `self.scoreboardRef` _returnvalue))
        (`UserWidget.AddToViewport` _output_get 0)
        (set `self.isWidgetOn` true)))))

(fn `UserConstructionScript`)