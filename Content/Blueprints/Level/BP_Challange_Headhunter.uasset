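; BP_Challange_Headhunter is an interactable level actor that switches a point light on and off, with no challenge logic despite its name.
; Focus toggles custom depth rendering on its Sphere, and interacting calls InteractOnServer to flip InteractToggle.
; The InteractToggle RepNotify sets the light's visibility to match.
; BeginPlay, the hit event and the widget getter are empty stubs, while Tick only stores the frame delta.
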(event `self.ReceiveBeginPlay`)

(event `self.ReceiveTick`
  (params (DeltaSeconds :type "Float (single-precision)"))
  (set `self.time` DeltaSeconds))

(event `/Game/Blueprints/BI_Interaction.Interface_ToggleFocus`
  (params (Focus :type Boolean))
  (`PrimitiveComponent.SetRenderCustomDepth` (`self.Sphere`) Focus))

(event `/Game/Blueprints/BI_Interaction.InterfaceInteract`
  (`self.InteractOnServer`))

(event `InteractOnServer`
  (set `self.interactToggle` (not (`self.interactToggle`))))

(event `self.Sphere.OnComponentHit`
  (params (HitComponent :type "PrimitiveComponent Object Reference") (OtherActor :type "Actor Object Reference") (OtherComp :type "PrimitiveComponent Object Reference") (NormalImpulse :type "Vector Structure") (Hit :type "HitResult Structure (by ref)")))

(fn `GetInteractionWidgetRef`
  (returns (Ref :type "WidgetComponent Object Reference"))
  (return null))

(fn `OnRep_interactToggle`
  (bind _pointlight (`self.PointLight`))
  (if (`self.interactToggle`)
    (`SceneComponent.SetVisibility` _pointlight true false)
    (else
      (`SceneComponent.SetVisibility` _pointlight false false))))

(fn `UserConstructionScript`
  (`parent.UserConstructionScript`))