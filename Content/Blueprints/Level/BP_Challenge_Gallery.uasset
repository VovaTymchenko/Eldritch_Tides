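; Shooting gallery challenge actor that runs a timed, scored round and pays the player money when it ends.
; Player overlap highlights the Sphere via custom depth and gates StartEvent, which spawns a skull through BP_Skull_Spawner and shows the WB_Challange widget.
; A one-second Delay loop counts down until Tick flags Defeat at zero.
; The widget then plays its end animation and closes, and the player receives triple the Score as money.
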(event `self.ReceiveActorBeginOverlap`
  (params (OtherActor :type "Actor Object Reference"))
  (if (== OtherActor (`GameplayStatics.GetPlayerCharacter` 0))
    (`PrimitiveComponent.SetRenderCustomDepth` (`self.Sphere`) true)
    (set `self.inInteractionZone` true)))

(event `self.ReceiveActorEndOverlap`
  (params (OtherActor :type "Actor Object Reference"))
  (if (== OtherActor (`GameplayStatics.GetPlayerCharacter` 0))
    (`PrimitiveComponent.SetRenderCustomDepth` (`self.Sphere`) false)
    (set `self.inInteractionZone` false)))

(event `Start Event`
  (if (`self.inInteractionZone`)
    (set `self.defeat` false)
    (bind _returnvalue (`GameplayStatics.GetActorOfClass` "/Game/Blueprints/Targets/BP_Skull_Spawner.BP_Skull_Spawner_C"))
    (bind _asbp_skull_spawner (cast `/Game/Blueprints/Targets/BP_Skull_Spawner` _returnvalue))
    (`/Game/Blueprints/Targets/BP_Skull_Spawner.Spawn_Skull` _asbp_skull_spawner)
    (bind _returnvalue_2 (`|CreateWidget` "/Game/UI/WB_Challange.WB_Challange_C"))
    (`UserWidget.AddToViewport` _returnvalue_2 0)
    (set `self.timeLeft` (`self.time`))
    (set `self.score` 0)
    (`KismetSystemLibrary.Delay` 1.0 :!label _label)
    (if (`self.defeat`)
      (`KismetSystemLibrary.PrintString` "DEFEAT!")
      (`UserWidget.PlayAnimation` _returnvalue_2 (`/Game/UI/WB_Challange.TheEnd` _returnvalue_2) 0.0 1 "Forward" 1.0 false)
      (`KismetSystemLibrary.Delay` 3.0)
      (`Widget.RemoveFromParent` _returnvalue_2)
      (bind _asbp_first_person_character (cast `/Game/Blueprints/BP_FirstPersonCharacter` (`GameplayStatics.GetPlayerCharacter` 0)))
      (set `/Game/Blueprints/BP_FirstPersonCharacter.Money` (+ (`/Game/Blueprints/BP_FirstPersonCharacter.Money` _asbp_first_person_character) (* (`self.score`) 3)) _asbp_first_person_character)
      (else
        (set `self.timeLeft` (- (`self.timeLeft`) 1.0))
        (goto _label)))))

(event `self.ReceiveTick`
  (params (DeltaSeconds :type "Float (single-precision)"))
  (if (<= (`self.timeLeft`) 0.0)
    (set `self.defeat` true)))

(fn `UserConstructionScript`)