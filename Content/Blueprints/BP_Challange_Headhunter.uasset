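; BP_Challange_Headhunter is an interactable actor that switches a point light on and off.
; Focus toggles custom depth rendering on its sphere, and it exposes a widget reference for interaction.
; Interacting calls InteractOnServer to flip InteractToggle, whose OnRep function sets the light's visibility to match.
; Tick only stores the frame delta in Time, and no headhunter challenge logic is present.
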(event `self.ReceiveBeginPlay`)

(event `self.ReceiveTick`
  (params (DeltaSeconds :type "Float (single-precision)"))
  (set `self.time` DeltaSeconds))

(event `/Game/Blueprints/BI_Interaction.Interface_ToggleFocus`
  (params (Focus :type Boolean))
  (`PrimitiveComponent.SetRenderCustomDepth` (`self.Sphere`) Focus))

(event `/Game/Blueprints/BI_Interaction.InterfaceInteract`
  (`self.InteractOnServer`))

(event `InteractOnServer`
  (set `self.interactToggle` (not (`self.interactToggle`))))

(fn `GetInteractionWidgetRef`
  (returns (Ref :type "WidgetComponent Object Reference"))
  (return (`self.Widget`)))

(fn `OnRep_interactToggle`
  (bind _pointlight (`self.PointLight`))
  (if (`self.interactToggle`)
    (`SceneComponent.SetVisibility` _pointlight true false)
    (else
      (`SceneComponent.SetVisibility` _pointlight false false))))

(fn `UserConstructionScript`
  (`parent.UserConstructionScript`))