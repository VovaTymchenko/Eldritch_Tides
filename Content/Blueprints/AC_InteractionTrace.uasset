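; Interaction component that detects BP_InteractionArea actors in the player's view and triggers interaction with them.
; Each tick, a camera line trace on the Visibility channel updates the focused area and toggles its focus.
; Interact input calls InteractOnServer, which messages the area's parent actor, immediately for zero-duration areas.
; Timed areas have widget progress and cancel-on-release logic, but the widget cast and looping timer setup are disconnected, so timed interactions never start.
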(event `self.ReceiveTick`
  (params (DeltaSeconds :type "Float (single-precision)"))
  (`self.Trace`))

(event `TryToInteract`
  (params (in :type Boolean))
  (if in
    (if (`self.isTracingInteractionArea`)
      (bind _output_get (set `self.Interact Duration` (`/Game/Blueprints/BP_InteractionArea.interactDuration` (`self.focusedInteractionArea`))))
      (if (> _output_get 0.0)
        (bind _ref (message `/Game/Blueprints/BI_Interaction.GetInteractionWidgetRef` (`Actor.GetParentActor` (`self.focusedInteractionArea`))))
        (else
          (`self.InteractOnServer` (`self.focusedInteractionArea`)))))
    (else
      (`self.StopInteraction`))))

(event `UpdateInteractionProgress`
  (bind _output_get (set `self.interactionProgress` (+ (* (/ 1.0 (`self.Interact Duration`)) (`self.updateInteractionInterval`)) (`self.interactionProgress`))))
  (`self.SetPercent` (`.currentInterractionWidgedRef` (`self.currentInterractionWidgedRef`)) _output_get)
  (if (>= (`self.interactionProgress`) 1.0)
    (`self.StopInteraction`)
    (`self.InteractOnServer` (`self.focusedInteractionArea`))))

(event `InteractOnServer`
  (params (InteractionArea :type "/Game/Blueprints/BP_InteractionArea Object Reference"))
  (message `/Game/Blueprints/BI_Interaction.InterfaceInteract` (`Actor.GetParentActor` InteractionArea)))

(fn `StopInteraction`
  (if (> (`self.interactionProgress`) 0.0)
    (`KismetSystemLibrary.K2_ClearAndInvalidateTimerHandle` (`self.interactionTimer`))
    (`self.SetPercent` (`.currentInterractionWidgedRef` (`self.currentInterractionWidgedRef`)) 0.0)
    (set `self.interactionProgress` 0.0)
    (set `self.currentInterractionWidgedRef` null)))

(fn `Trace`
  (bind _returnvalue (`GameplayStatics.GetPlayerCameraManager` 0))
  (bind _returnvalue_2 (`Actor.K2_GetActorLocation` _returnvalue))
  (bind (_outhit _returnvalue_3) (`KismetSystemLibrary.LineTraceSingle` _returnvalue_2 (+ _returnvalue_2 (* (`KismetMathLibrary.GetForwardVector` (`Actor.K2_GetActorRotation` _returnvalue)) (`self.interactionMaxDistance`))) "TraceTypeQuery1"))
  (if _returnvalue_3
    (bind (_bblockinghit _binitialoverlap _time _distance _location _impactpoint _normal _impactnormal _physmat _hitactor) (`GameplayStatics.BreakHitResult` _outhit))
    (if (!= (`self.focusedActor`) _hitactor)
      (set `self.focusedActor` _hitactor)
      (`self.TraceInteractionArea` (== (`GameplayStatics.GetObjectClass` _hitactor) "/Game/Blueprints/BP_InteractionArea.BP_InteractionArea_C")))
    (else
      (`self.TraceInteractionArea` false))))

(fn `TraceInteractionArea`
  (params (Trace :type Boolean))
  (if Trace
    (if (`self.isTracingInteractionArea`)
      (`/Game/Blueprints/BP_InteractionArea.Toggle Focus` (`self.focusedInteractionArea`) false))
    (bind _asbp_interaction_area (cast `/Game/Blueprints/BP_InteractionArea` (`self.focusedActor`)))
    (bind _output_get (set `self.focusedInteractionArea` _asbp_interaction_area))
    (`/Game/Blueprints/BP_InteractionArea.Toggle Focus` _output_get true)
    (set `self.isTracingInteractionArea` true)
    (elif (`self.isTracingInteractionArea`)
      (set `self.isTracingInteractionArea` false)
      (`/Game/Blueprints/BP_InteractionArea.Toggle Focus` (`self.focusedInteractionArea`) false)
      (set `self.focusedActor` null)
      (set `self.focusedInteractionArea` null))))