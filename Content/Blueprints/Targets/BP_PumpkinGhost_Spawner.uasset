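; Spawner actor that continuously spawns BP_Target_PumpkinGhost targets at random points on a ring around itself.
; BeginPlay starts spawning, then offsets eight sphere components by Distance along the axes and diagonals to form the ring.
; The spawn event picks a random sphere, spawns a ghost at its world location, then loops after a short Delay with no stop condition.
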(event `self.ReceiveBeginPlay`
  (bind _returnvalue (`KismetMathLibrary.Sqrt` (* (`KismetMathLibrary.Square` (`self.Distance`)) 0.5)))
  (bind _returnvalue_2 (`KismetMathLibrary.Sqrt` (* (`KismetMathLibrary.Square` (`self.Distance`)) 0.5)))
  (bind _returnvalue_3 (`KismetMathLibrary.Sqrt` (* (`KismetMathLibrary.Square` (`self.Distance`)) 0.5)))
  (bind _returnvalue_4 (- 0.0 (`KismetMathLibrary.Sqrt` (* (`KismetMathLibrary.Square` (`self.Distance`)) 0.5))))
  (`self.Spawn_PumpkinGhost`)
  (`|ExecutionSequence`
    (:`then_0`
      (`SceneComponent.K2_AddLocalOffset` (`self.Sphere`) (`KismetMathLibrary.MakeVector` (`self.Distance`)) false true))
    (:`then_1`
      (`SceneComponent.K2_AddLocalOffset` (`self.Sphere1`) (`KismetMathLibrary.MakeVector` (- 0.0 (`self.Distance`))) false true))
    (:`then_2`
      (`SceneComponent.K2_AddLocalOffset` (`self.Sphere2`) (`KismetMathLibrary.MakeVector` 0.0 (`self.Distance`)) false true))
    (:`then_3`
      (`SceneComponent.K2_AddLocalOffset` (`self.Sphere3`) (`KismetMathLibrary.MakeVector` 0.0 (- 0.0 (`self.Distance`))) false true))
    (:`then_4`
      (`SceneComponent.K2_AddLocalOffset` (`self.Sphere4`) (`KismetMathLibrary.MakeVector` _returnvalue_3 _returnvalue_3) false true))
    (:`then_5`
      (`SceneComponent.K2_AddLocalOffset` (`self.Sphere5`) (`KismetMathLibrary.MakeVector` _returnvalue_4 _returnvalue_4) false true))
    (:`then_6`
      (`SceneComponent.K2_AddLocalOffset` (`self.Sphere6`) (`KismetMathLibrary.MakeVector` (- 0.0 _returnvalue_2) _returnvalue_2) false true))
    (:`then_7`
      (`SceneComponent.K2_AddLocalOffset` (`self.Sphere7`) (`KismetMathLibrary.MakeVector` _returnvalue (- 0.0 _returnvalue)) false true))))

(event `Spawn_PumpkinGhost`
  (switch `int` (`KismetMathLibrary.RandomIntegerInRange` 0 7) :!label _label
    (:`0`
      (`|SpawnActorFromClass` "/Game/Blueprints/Targets/BP_Target_PumpkinGhost.BP_Target_PumpkinGhost_C" (`KismetMathLibrary.MakeTransform` (`SceneComponent.K2_GetComponentLocation` (`self.Sphere`))) "Undefined" "OverrideRootScale" null null))
    (:`1`
      (`|SpawnActorFromClass` "/Game/Blueprints/Targets/BP_Target_PumpkinGhost.BP_Target_PumpkinGhost_C" (`KismetMathLibrary.MakeTransform` (`SceneComponent.K2_GetComponentLocation` (`self.Sphere1`))) "Undefined" "OverrideRootScale" null null))
    (:`2`
      (`|SpawnActorFromClass` "/Game/Blueprints/Targets/BP_Target_PumpkinGhost.BP_Target_PumpkinGhost_C" (`KismetMathLibrary.MakeTransform` (`SceneComponent.K2_GetComponentLocation` (`self.Sphere2`))) "Undefined" "OverrideRootScale" null null))
    (:`3`
      (`|SpawnActorFromClass` "/Game/Blueprints/Targets/BP_Target_PumpkinGhost.BP_Target_PumpkinGhost_C" (`KismetMathLibrary.MakeTransform` (`SceneComponent.K2_GetComponentLocation` (`self.Sphere3`))) "Undefined" "OverrideRootScale" null null))
    (:`4`
      (`|SpawnActorFromClass` "/Game/Blueprints/Targets/BP_Target_PumpkinGhost.BP_Target_PumpkinGhost_C" (`KismetMathLibrary.MakeTransform` (`SceneComponent.K2_GetComponentLocation` (`self.Sphere4`))) "Undefined" "OverrideRootScale" null null))
    (:`5`
      (`|SpawnActorFromClass` "/Game/Blueprints/Targets/BP_Target_PumpkinGhost.BP_Target_PumpkinGhost_C" (`KismetMathLibrary.MakeTransform` (`SceneComponent.K2_GetComponentLocation` (`self.Sphere5`))) "Undefined" "OverrideRootScale" null null))
    (:`6`
      (`|SpawnActorFromClass` "/Game/Blueprints/Targets/BP_Target_PumpkinGhost.BP_Target_PumpkinGhost_C" (`KismetMathLibrary.MakeTransform` (`SceneComponent.K2_GetComponentLocation` (`self.Sphere6`))) "Undefined" "OverrideRootScale" null null))
    (:`7`
      (`|SpawnActorFromClass` "/Game/Blueprints/Targets/BP_Target_PumpkinGhost.BP_Target_PumpkinGhost_C" (`KismetMathLibrary.MakeTransform` (`SceneComponent.K2_GetComponentLocation` (`self.Sphere7`))) "Undefined" "OverrideRootScale" null null)))
  (`KismetSystemLibrary.Delay` 0.2)
  (goto _label))

(fn `UserConstructionScript`)