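; Spawner that places a wave of BP_Target_Skull targets at marker components each time its Spawn_Skull event runs.
; Sixteen Sphere components form eight pairs, and a chain of coin flips picks one location from each pair, so every call spawns eight skulls in a random layout.
; Both branches of each flip rejoin before the next pair, and skulls spawn with zero rotation and unit scale.
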(event `Spawn_Skull`
  (switch `int` (`KismetMathLibrary.RandomIntegerInRange` 0 1)
    (:`0`
      (`|SpawnActorFromClass` "/Game/Blueprints/Targets/BP_Target_Skull.BP_Target_Skull_C" (`KismetMathLibrary.MakeTransform` (`SceneComponent.K2_GetComponentLocation` (`self.Sphere`))) "Undefined" "OverrideRootScale" null null))
    (:`1`
      (`|SpawnActorFromClass` "/Game/Blueprints/Targets/BP_Target_Skull.BP_Target_Skull_C" (`KismetMathLibrary.MakeTransform` (`SceneComponent.K2_GetComponentLocation` (`self.Sphere1`))) "Undefined" "OverrideRootScale" null null)))
  (switch `int` (`KismetMathLibrary.RandomIntegerInRange` 0 1)
    (:`0`
      (`|SpawnActorFromClass` "/Game/Blueprints/Targets/BP_Target_Skull.BP_Target_Skull_C" (`KismetMathLibrary.MakeTransform` (`SceneComponent.K2_GetComponentLocation` (`self.Sphere2`))) "Undefined" "OverrideRootScale" null null))
    (:`1`
      (`|SpawnActorFromClass` "/Game/Blueprints/Targets/BP_Target_Skull.BP_Target_Skull_C" (`KismetMathLibrary.MakeTransform` (`SceneComponent.K2_GetComponentLocation` (`self.Sphere3`))) "Undefined" "OverrideRootScale" null null)))
  (switch `int` (`KismetMathLibrary.RandomIntegerInRange` 0 1)
    (:`0`
      (`|SpawnActorFromClass` "/Game/Blueprints/Targets/BP_Target_Skull.BP_Target_Skull_C" (`KismetMathLibrary.MakeTransform` (`SceneComponent.K2_GetComponentLocation` (`self.Sphere4`))) "Undefined" "OverrideRootScale" null null))
    (:`1`
      (`|SpawnActorFromClass` "/Game/Blueprints/Targets/BP_Target_Skull.BP_Target_Skull_C" (`KismetMathLibrary.MakeTransform` (`SceneComponent.K2_GetComponentLocation` (`self.Sphere5`))) "Undefined" "OverrideRootScale" null null)))
  (switch `int` (`KismetMathLibrary.RandomIntegerInRange` 0 1)
    (:`0`
      (`|SpawnActorFromClass` "/Game/Blueprints/Targets/BP_Target_Skull.BP_Target_Skull_C" (`KismetMathLibrary.MakeTransform` (`SceneComponent.K2_GetComponentLocation` (`self.Sphere6`))) "Undefined" "OverrideRootScale" null null))
    (:`1`
      (`|SpawnActorFromClass` "/Game/Blueprints/Targets/BP_Target_Skull.BP_Target_Skull_C" (`KismetMathLibrary.MakeTransform` (`SceneComponent.K2_GetComponentLocation` (`self.Sphere7`))) "Undefined" "OverrideRootScale" null null)))
  (switch `int` (`KismetMathLibrary.RandomIntegerInRange` 0 1)
    (:`0`
      (`|SpawnActorFromClass` "/Game/Blueprints/Targets/BP_Target_Skull.BP_Target_Skull_C" (`KismetMathLibrary.MakeTransform` (`SceneComponent.K2_GetComponentLocation` (`self.Sphere8`))) "Undefined" "OverrideRootScale" null null))
    (:`1`
      (`|SpawnActorFromClass` "/Game/Blueprints/Targets/BP_Target_Skull.BP_Target_Skull_C" (`KismetMathLibrary.MakeTransform` (`SceneComponent.K2_GetComponentLocation` (`self.Sphere9`))) "Undefined" "OverrideRootScale" null null)))
  (switch `int` (`KismetMathLibrary.RandomIntegerInRange` 0 1)
    (:`0`
      (`|SpawnActorFromClass` "/Game/Blueprints/Targets/BP_Target_Skull.BP_Target_Skull_C" (`KismetMathLibrary.MakeTransform` (`SceneComponent.K2_GetComponentLocation` (`self.Sphere10`))) "Undefined" "OverrideRootScale" null null))
    (:`1`
      (`|SpawnActorFromClass` "/Game/Blueprints/Targets/BP_Target_Skull.BP_Target_Skull_C" (`KismetMathLibrary.MakeTransform` (`SceneComponent.K2_GetComponentLocation` (`self.Sphere11`))) "Undefined" "OverrideRootScale" null null)))
  (switch `int` (`KismetMathLibrary.RandomIntegerInRange` 0 1)
    (:`0`
      (`|SpawnActorFromClass` "/Game/Blueprints/Targets/BP_Target_Skull.BP_Target_Skull_C" (`KismetMathLibrary.MakeTransform` (`SceneComponent.K2_GetComponentLocation` (`self.Sphere12`))) "Undefined" "OverrideRootScale" null null))
    (:`1`
      (`|SpawnActorFromClass` "/Game/Blueprints/Targets/BP_Target_Skull.BP_Target_Skull_C" (`KismetMathLibrary.MakeTransform` (`SceneComponent.K2_GetComponentLocation` (`self.Sphere13`))) "Undefined" "OverrideRootScale" null null)))
  (switch `int` (`KismetMathLibrary.RandomIntegerInRange` 0 1)
    (:`0`
      (`|SpawnActorFromClass` "/Game/Blueprints/Targets/BP_Target_Skull.BP_Target_Skull_C" (`KismetMathLibrary.MakeTransform` (`SceneComponent.K2_GetComponentLocation` (`self.Sphere14`))) "Undefined" "OverrideRootScale" null null))
    (:`1`
      (`|SpawnActorFromClass` "/Game/Blueprints/Targets/BP_Target_Skull.BP_Target_Skull_C" (`KismetMathLibrary.MakeTransform` (`SceneComponent.K2_GetComponentLocation` (`self.Sphere15`))) "Undefined" "OverrideRootScale" null null))))

(fn `UserConstructionScript`)