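; Thrown flashbang actor that launches from the first-person player's view and detonates after a short fuse.
; On BeginPlay it applies an impulse along the camera forward vector to its static mesh, plus a random angular impulse for spin.
; After a fixed delay it spawns an explosion decal, calls Flashbang on the player character with distance and mesh location, then destroys itself.
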(event `self.ReceiveBeginPlay`
  (bind _staticmesh (`self.StaticMesh`))
  (bind _returnvalue (`SceneComponent.K2_GetComponentLocation` _staticmesh))
  (bind _asbp_first_person_character (cast `/Game/FirstPerson/Blueprints/BP_FirstPersonCharacter` (`GameplayStatics.GetPlayerPawn` 0)))
  (`PrimitiveComponent.AddImpulse` _staticmesh (* (`SceneComponent.GetForwardVector` (`/Game/FirstPerson/Blueprints/BP_FirstPersonCharacter.FirstPersonCamera` _asbp_first_person_character)) 1500.0) "None" true)
  (`PrimitiveComponent.AddAngularImpulseInDegrees` _staticmesh (* (`KismetMathLibrary.RandomUnitVector`) 350.0) "None" false)
  (`KismetSystemLibrary.Delay` 3.0)
  (`|SpawnActorFromClass` "/Game/Flash_Spell/ExplosionDecal_BP.ExplosionDecal_BP_C" (`KismetMathLibrary.MakeTransform` _returnvalue (struct :`Pitch` 90.0)) "Undefined" "OverrideRootScale" null null)
  (`/Game/FirstPerson/Blueprints/BP_FirstPersonCharacter.Flashbang` _asbp_first_person_character (`self.GetDistanceTo` _asbp_first_person_character null) _returnvalue)
  (`self.K2_DestroyActor`))

(fn `UserConstructionScript`)